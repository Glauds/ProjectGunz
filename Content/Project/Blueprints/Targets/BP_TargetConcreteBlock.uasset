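; BP_TargetConcreteBlock is a concrete block target with a normal mesh and a Chaos destructible wall.
; On BeginPlay it reads the mass from the wall's geometry collection and applies it as a mass override to both the normal mesh and the Chaos wall, keeping their physical weight matched.
; It reports its target location as the Chaos wall's world position.
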(event `self.ReceiveBeginPlay`
  (bind _chaos_wall (`self.Chaos_Wall`))
  ;[1 1 1] Ustawienie masy do takiej co ma sciana na chaosie
  (`parent.ReceiveBeginPlay`)
  (bind _output_get (set `self.Mass` (`GeometryCollection.Mass` (`GeometryCollectionComponent.RestCollection` _chaos_wall))))
  (`PrimitiveComponent.SetMassOverrideInKg` (`self.NormalMesh`) "None" _output_get true)
  (`PrimitiveComponent.SetMassOverrideInKg` _chaos_wall "None" _output_get true))

(fn `Get Target Location`
  (returns (ReturnValue :type "Vector Structure"))
  (return (`SceneComponent.K2_GetComponentLocation` (`self.Chaos_Wall`))))

(fn `UserConstructionScript`
  (`parent.UserConstructionScript`))