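; Player controller that handles pausing and unpausing the game through a pause menu widget.
; The Pause input only opens the menu, creating WBP_PauseMenu, focusing it in UI-only input mode with a visible cursor, and pausing the game.
; TogglePause with false removes and clears the widget, restores game-only input with permanent mouse capture and hidden cursor, then unpauses.
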(event `InputAction|Pause`
  (params (Key :type "Key Structure"))
  (:`Pressed`
    (`self.TogglePause` true)))

(event `TogglePause`
  (params (IsPause :type Boolean))
  (if IsPause
    (bind _returnvalue (`|CreateWidget` "/Game/Project/Blueprints/Widgets/Menu/WBP_PauseMenu.WBP_PauseMenu_C" self))
    (bind _output_get (set `self.PauseMenuRef` _returnvalue))
    (`UserWidget.AddToViewport` _output_get 0)
    (`self.UI Only` self _returnvalue)
    (`GameplayStatics.SetGamePaused` true)
    (else
      (`Widget.RemoveFromParent` (`self.PauseMenuRef`))
      (`self.GameOnly`)
      (`GameplayStatics.SetGamePaused` false)
      (set `self.PauseMenuRef` null))))

(event `UI Only`
  (params (WidgetToFocus :type "Widget Object Reference"))
  (`WidgetBlueprintLibrary.SetInputMode_UIOnlyEx` self WidgetToFocus)
  (set `self.bShowMouseCursor` true))

(event `GameOnly`
  (`WidgetBlueprintLibrary.SetInputMode_GameOnly` self)
  (`GameplayStatics.SetViewportMouseCaptureMode` "CapturePermanently_IncludingInitialMouseDown")
  (set `self.bShowMouseCursor` false))

(fn `UserConstructionScript`)