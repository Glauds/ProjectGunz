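; Game instance that persists player options and provides display toggles for HDR and post-processing.
; On Init, after a short delay, it creates the OptionsSave slot if missing, then applies the saved scalability level and stores effects volume.
; A save event writes both values back to the slot.
; HDR switches through console commands with color gamut and output device helpers, while post-processing flips Enabled on an array of volumes.
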(event `self.ReceiveInit`
  (`KismetSystemLibrary.Delay` 0.2)
  (bind _returnvalue (`GameplayStatics.DoesSaveGameExist` (`self.OptionsSave`)))
  (if _returnvalue
    (`self.LoadGameSettings`)
    (else
      (`self.CreateGameSettingsSave`)
      (`self.LoadGameSettings`))))

(event `CreateGameSettingsSave`
  (bind _returnvalue (`GameplayStatics.CreateSaveGameObject` "/Game/Project/Blueprints/Core/Menu/BP_OptionsSave.BP_OptionsSave_C"))
  (`GameplayStatics.SaveGameToSlot` _returnvalue (`self.OptionsSave`)))

(event `LoadGameSettings`
  (bind _returnvalue (`GameplayStatics.LoadGameFromSlot` (`self.OptionsSave`)))
  (bind _asbp_options_save (cast `/Game/Project/Blueprints/Core/Menu/BP_OptionsSave` _returnvalue))
  (bind _returnvalue_2 (`GameUserSettings.GetGameUserSettings`))
  (`GameUserSettings.SetOverallScalabilityLevel` _returnvalue_2 (`/Game/Project/Blueprints/Core/Menu/BP_OptionsSave.GraphicLevel` _asbp_options_save))
  (`GameUserSettings.ApplySettings` _returnvalue_2 true)
  (set `self.EffectsVolume` (`/Game/Project/Blueprints/Core/Menu/BP_OptionsSave.EffectsVolume` _asbp_options_save)))

(event `SaveGameSettings`
  (bind _returnvalue (`GameplayStatics.LoadGameFromSlot` (`self.OptionsSave`)))
  (bind _asbp_options_save (cast `/Game/Project/Blueprints/Core/Menu/BP_OptionsSave` _returnvalue))
  (bind _returnvalue_2 (`GameUserSettings.GetGameUserSettings`))
  (set `/Game/Project/Blueprints/Core/Menu/BP_OptionsSave.GraphicLevel` (`GameUserSettings.GetOverallScalabilityLevel` _returnvalue_2) _asbp_options_save)
  (set `/Game/Project/Blueprints/Core/Menu/BP_OptionsSave.EffectsVolume` (`self.EffectsVolume`) _asbp_options_save)
  (`GameplayStatics.SaveGameToSlot` _asbp_options_save (`self.OptionsSave`)))

(event `ToggleHDR`
  ;[1 1 1] HDR
  (bind _returnvalue (`KismetSystemLibrary.GetConsoleVariableBoolValue` "r.HDR.EnableHDROutput"))
  (if _returnvalue
    (`KismetSystemLibrary.ExecuteConsoleCommand` "r.HDR.EnableHDROutput 0" null)
    (`KismetSystemLibrary.ExecuteConsoleCommand` "r.HDR.UI.CompositeMode 0" null)
    (`KismetSystemLibrary.ExecuteConsoleCommand` "r.HDR.UI.Level 0" null)
    (`self.SetHDRColorGamut` 0)
    (`self.SetHDRDevice` 0)
    (else
      (`KismetSystemLibrary.ExecuteConsoleCommand` "r.HDR.EnableHDROutput 1" null)
      (`KismetSystemLibrary.ExecuteConsoleCommand` "r.HDR.UI.CompositeMode 1" null)
      (`KismetSystemLibrary.ExecuteConsoleCommand` "r.HDR.UI.Level 2" null)
      (`self.SetHDRColorGamut` 0)
      (`self.SetHDRDevice` 5))))

(event `SetHDRColorGamut`
  (params (ColorGamut :type Integer))
  ;[1 1 1] HDR Gama kolorów
  (`KismetSystemLibrary.ExecuteConsoleCommand` (`KismetStringLibrary.Concat_StrStr` "r.HDR.Display.ColorGamut " (`KismetStringLibrary.Conv_IntToString` ColorGamut)) null))

(event `SetHDRDevice`
  (params (Device :type Integer))
  ;[1 1 1] HDR wyswietlacz
  (`KismetSystemLibrary.ExecuteConsoleCommand` (`KismetStringLibrary.Concat_StrStr` "r.HDR.Display.OutputDevice " (`KismetStringLibrary.Conv_IntToString` Device)) null))

(event `TogglePostProcess`
  ;[1 1 1] Postprocessy
  (set `self.PostProcess` (not (`self.PostProcess`)))
  (for _array_element (`self.PostProcessVolumes`)
    (set `PostProcessVolume.bEnabled` (`self.PostProcess`) _array_element)))