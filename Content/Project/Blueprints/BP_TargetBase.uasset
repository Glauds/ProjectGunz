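; BP_TargetBase is a base target actor that shows a camera view of an incoming projectile shot.
; When a BP_ProjectileBase enters its camera trigger box, it clears CanBeTarget and cuts the first player's view to TargetCamera.
; After WatchTime, the view eases back to the controlled pawn over BackTime.
; Once that blend time elapses, it calls AllowFiring on that pawn if it is a BP_VehicleBase.
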(event `self.CameraTriggerBox.OnComponentBeginOverlap`
  (params (OverlappedComponent :type "PrimitiveComponent Object Reference") (OtherActor :type "Actor Object Reference") (OtherComp :type "PrimitiveComponent Object Reference") (OtherBodyIndex :type Integer) (bFromSweep :type Boolean) (SweepResult :type "HitResult Structure (by ref)"))
  (bind _returnvalue (`GameplayStatics.GetPlayerController` 0))
  (bind _returnvalue_2 (`Controller.K2_GetPawn` _returnvalue))
  (cast `/Game/Project/Blueprints/BP_ProjectileBase` OtherActor)
  (set `self.CanBeTarget` false)
  ;[1 1 1] Ogladanie
  (`PlayerController.SetViewTargetWithBlend` (`GameplayStatics.GetPlayerController` 0) (`self.TargetCamera`) 0.0 "VTBlend_Linear" 0.0 false)
  ;[1 1 1] Powrot do pojazdu
  (`KismetSystemLibrary.Delay` (`self.WatchTime`))
  (`PlayerController.SetViewTargetWithBlend` _returnvalue _returnvalue_2 (`self.BackTime`) "VTBlend_EaseOut" 2.0 false)
  (`KismetSystemLibrary.Delay` (`self.BackTime`))
  (bind _asbp_vehicle_base (cast `/Game/Project/Blueprints/BP_VehicleBase` _returnvalue_2))
  (`/Game/Project/Blueprints/BP_VehicleBase.AllowFiring` _asbp_vehicle_base null))

(fn `UserConstructionScript`)