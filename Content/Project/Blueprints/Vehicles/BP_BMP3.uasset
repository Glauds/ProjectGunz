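; BP_BMP3 is a BMP-3 vehicle Blueprint that aims its turret at a target actor.
; The RotatetoTarget event eases the Turret component over two seconds to the look-at yaw toward TargetActor, keeping pitch and roll.
; It then stores the location and rotation of the turret's Projectile socket, so muzzle placement can come from the model rather than the logic.
; Nothing in this graph calls the event or spawns a projectile.
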(event `self.RotateToTarget`
  (bind _turret (`self.Turret`))
  (bind (_relativerotation_roll _relativerotation_pitch) (`KismetMathLibrary.BreakRotator` (`SceneComponent.RelativeRotation` _turret)))
  (bind (_returnvalue_roll _returnvalue_pitch _returnvalue_yaw) (`KismetMathLibrary.BreakRotator` (`KismetMathLibrary.FindLookAtRotation` (`SceneComponent.K2_GetComponentLocation` (`self.Turret`)) (`self.K2_GetActorLocation` (`self.Target Actor`)))))
  (`KismetSystemLibrary.MoveComponentTo` _turret (`SceneComponent.RelativeLocation` _turret) (`KismetMathLibrary.MakeRotator` _relativerotation_roll _relativerotation_pitch _returnvalue_yaw) false true 2.0)
  (set `self.ProjectileLocation` (`SceneComponent.GetSocketLocation` (`self.Turret`) "Projectile"))
  (set `self.ProjectileRotation` (`SceneComponent.GetSocketRotation` (`self.Turret`) "Projectile")))

(fn `UserConstructionScript`
  (`parent.UserConstructionScript`))