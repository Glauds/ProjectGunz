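; BP_M777 is an artillery piece, named for the M777 howitzer, that turns to face a target actor.
; A RotatetoTarget event eases the capsule's yaw toward TargetActor over a short timed MoveComponentTo, keeping its pitch and roll.
; It then stores the mesh's Projectile socket location in ProjectileLocation, so the launch point comes from the model.
; The file contains no firing logic, and its BeginPlay, overlap and Tick events are disabled.
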(event `self.RotateToTarget`
  (bind _capsulecomponent (`self.CapsuleComponent`))
  (bind (_relativerotation_roll _relativerotation_pitch) (`KismetMathLibrary.BreakRotator` (`SceneComponent.RelativeRotation` _capsulecomponent)))
  (bind (_returnvalue_roll _returnvalue_pitch _returnvalue_yaw) (`KismetMathLibrary.BreakRotator` (`KismetMathLibrary.FindLookAtRotation` (`self.K2_GetActorLocation`) (`self.K2_GetActorLocation` (`self.Target Actor`)))))
  (`KismetSystemLibrary.MoveComponentTo` _capsulecomponent (`SceneComponent.RelativeLocation` _capsulecomponent) (`KismetMathLibrary.MakeRotator` _relativerotation_roll _relativerotation_pitch _returnvalue_yaw) false true 2.0)
  (set `self.ProjectileLocation` (`SceneComponent.GetSocketLocation` (`self.Mesh`) "Projectile")))

(fn `UserConstructionScript`
  (`parent.UserConstructionScript`))